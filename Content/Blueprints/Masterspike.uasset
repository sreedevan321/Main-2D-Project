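; Masterspike is a 2D spike trap that cycles up and down and damages actors that begin overlapping its box.
; BeginPlay runs an endless loop that alternates the lower and raise events, waiting a short fixed delay plus a Duration variable after each.
; Each event steps through four Paper2D sprites with delays, then switches box collision off when lowered or on when raised.
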(event `self.ReceiveBeginPlay`
  (`parent.ReceiveBeginPlay`)
  (`self.Bringspikesdown` :!label _label)
  (`KismetSystemLibrary.Delay` 0.4)
  (`KismetSystemLibrary.Delay` (`self.Duration`))
  (`self.Bringspikesup`)
  (`KismetSystemLibrary.Delay` 0.4)
  (`KismetSystemLibrary.Delay` (`self.Duration`))
  (goto _label))

(event `Bringspikesdown`
  (`PaperSpriteComponent.SetSprite` (`self.PaperSprite`) "/Game/Assets/spikes/spike1_Sprite.spike1_Sprite")
  (`KismetSystemLibrary.Delay` 0.1)
  (`PaperSpriteComponent.SetSprite` (`self.PaperSprite`) "/Game/Assets/spikes/spike2_Sprite.spike2_Sprite")
  (`KismetSystemLibrary.Delay` 0.2)
  (`PaperSpriteComponent.SetSprite` (`self.PaperSprite`) "/Game/Assets/spikes/spike3_Sprite.spike3_Sprite")
  (`KismetSystemLibrary.Delay` 0.2)
  (`PaperSpriteComponent.SetSprite` (`self.PaperSprite`) "/Game/Assets/spikes/spike4_Sprite.spike4_Sprite")
  (`PrimitiveComponent.SetCollisionEnabled` (`self.Box`) "NoCollision"))

(event `Bringspikesup`
  (`PaperSpriteComponent.SetSprite` (`self.PaperSprite`) "/Game/Assets/spikes/spike4_Sprite.spike4_Sprite")
  (`KismetSystemLibrary.Delay` 0.1)
  (`PaperSpriteComponent.SetSprite` (`self.PaperSprite`) "/Game/Assets/spikes/spike3_Sprite.spike3_Sprite")
  (`KismetSystemLibrary.Delay` 0.2)
  (`PaperSpriteComponent.SetSprite` (`self.PaperSprite`) "/Game/Assets/spikes/spike2_Sprite.spike2_Sprite")
  (`KismetSystemLibrary.Delay` 0.2)
  (`PaperSpriteComponent.SetSprite` (`self.PaperSprite`) "/Game/Assets/spikes/spike1_Sprite.spike1_Sprite")
  (`PrimitiveComponent.SetCollisionEnabled` (`self.Box`) "QueryAndPhysics"))

(event `self.Box.OnComponentBeginOverlap`
  (params (OverlappedComponent :type "PrimitiveComponent Object Reference") (OtherActor :type "Actor Object Reference") (OtherComp :type "PrimitiveComponent Object Reference") (OtherBodyIndex :type Integer) (bFromSweep :type Boolean) (SweepResult :type "HitResult Structure (by ref)"))
  (`GameplayStatics.ApplyDamage` OtherActor 1.0))

(fn `UserConstructionScript`
  (`parent.UserConstructionScript`))