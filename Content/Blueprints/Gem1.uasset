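; Gem1 is a gem pickup actor that triggers the win screen when its Box component is overlapped.
; The overlap clears the timer on the player character's HUD, waits briefly, then destroys the gem, shows the WinUI widget with UI-only input and mouse cursor, and plays a power-up sound.
; The player check is left unconnected and the branch is always true, so any overlapping actor triggers the win.
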(event `self.Box.OnComponentBeginOverlap`
  (params (OverlappedComponent :type "PrimitiveComponent Object Reference") (OtherActor :type "Actor Object Reference") (OtherComp :type "PrimitiveComponent Object Reference") (OtherBodyIndex :type Integer) (bFromSweep :type Boolean) (SweepResult :type "HitResult Structure (by ref)"))
  (bind _returnvalue (`GameplayStatics.GetPlayerController` 0))
  ;[1 1 1] Comment
  (if true
    (`KismetSystemLibrary.K2_ClearAndInvalidateTimerHandle` (`/Game/UI/Playerhud.TIMEREVENT` (`/Game/Blueprints/2dPlayerCharacter.Playerhud` (`self.Playercharacterref`))))
    (`KismetSystemLibrary.Delay` 0.5)
    (`self.K2_DestroyActor`)
    (bind _returnvalue_2 (`|CreateWidget` "/Game/UI/WinUI.WinUI_C"))
    (`UserWidget.AddToViewport` _returnvalue_2 0)
    (`WidgetBlueprintLibrary.SetInputMode_UIOnlyEx` _returnvalue null)
    (set `PlayerController.bShowMouseCursor` true _returnvalue)
    (`GameplayStatics.PlaySound2D` "/Game/sounds/power_up.power_up" 1.0 1.0 0.0 null null)))

(fn `UserConstructionScript`
  (`parent.UserConstructionScript`))