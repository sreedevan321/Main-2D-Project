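; Health pickup actor that heals the 2D player character by a fixed amount and then destroys itself.
; The Box component's begin-overlap event casts player zero's character to 2dPlayerCharacter, adds to its Health and removes the pickup.
; The overlapping actor is never checked, so any overlap triggers the heal, and Health is not clamped here.
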(event `self.Box.OnComponentBeginOverlap`
  (params (OverlappedComponent :type "PrimitiveComponent Object Reference") (OtherActor :type "Actor Object Reference") (OtherComp :type "PrimitiveComponent Object Reference") (OtherBodyIndex :type Integer) (bFromSweep :type Boolean) (SweepResult :type "HitResult Structure (by ref)"))
  (bind _as2d_player_character (cast `/Game/Blueprints/2dPlayerCharacter` (`GameplayStatics.GetPlayerCharacter` 0)))
  (set `/Game/Blueprints/2dPlayerCharacter.health ` (+ (`/Game/Blueprints/2dPlayerCharacter.health ` _as2d_player_character) 25.0) _as2d_player_character)
  (`self.K2_DestroyActor`))

(fn `UserConstructionScript`
  (`parent.UserConstructionScript`))