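; Player character for a 2D side-scroller with jumping, horizontal movement, HUD, music and respawning at its start location.
; Tick picks the flipbook from death, falling and velocity, and flips control yaw by travel direction.
; Any damage freezes movement for the death animation, then respawns the player and subtracts health.
; The death flipbook switch also plays a hurt sound, self-applies damage and shows the lose screen at zero health.
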(event `self.ReceiveTick`
  (params (DeltaSeconds :type "Float (single-precision)"))
  ;[1 1 1] Event tick
  (`self.Handle Animation`)
  (`self.HandleRotation`))

(event `InputAction|Jump`
  (params (Key :type "Key Structure"))
  ;[1 1 1] Handle jumping
  (:`Pressed`
    (`self.Jump`)
    (`GameplayStatics.PlaySound2D` "/Game/sounds/jump.jump" 1.0 1.0 0.0 null null))
  (:`Released`
    (`self.StopJumping`)))

(event `InputAxis|Moveright`
  (params (AxisValue :type "Float (single-precision)"))
  ;[1 1 1] Handle Movement
  (if (> AxisValue 0.0)
    (set `self.ismovingright` true)
    (elif (< AxisValue 0.0)
      (set `self.ismovingright` false)))
  (`self.AddMovementInput` (1.0 0.0 0.0) AxisValue))

(event `Handle Animation`
  (bind _returnvalue (`GameplayStatics.GetPlayerController` 0))
  (bind _sprite (`self.Sprite`))
  ;[1 1 1] Handle Animation
  (if (`self.isdeath`)
    (bind _returnvalue_2 (`PaperFlipbookComponent.SetFlipbook` (`self.Sprite`) (`self.playerdeathanimation`)))
    (if _returnvalue_2
      (`KismetSystemLibrary.Delay` 0.2)
      (`GameplayStatics.PlaySound2D` "/Game/sounds/hurt.hurt" 1.0 1.0 0.0 null null)
      (`GameplayStatics.ApplyDamage` self 10.0)
      (if (== (`self.health `) 0.0)
        (bind _returnvalue_3 (`|CreateWidget` "/Game/UI/LoseUI1.LoseUI1_C"))
        (`UserWidget.AddToViewport` _returnvalue_3 0)
        (`WidgetBlueprintLibrary.SetInputMode_UIOnlyEx` _returnvalue null)
        (set `PlayerController.bShowMouseCursor` true _returnvalue)))
    (elif (`NavMovementComponent.IsFalling` (`self.CharacterMovement`))
      (`PaperFlipbookComponent.SetFlipbook` _sprite "/Game/Assets/Characters/Jump.Jump")
      (else
        (`PaperFlipbookComponent.SetFlipbook` _sprite (select `bool` (> (`KismetMathLibrary.VSize` (`MovementComponent.Velocity` (`self.CharacterMovement`))) 0.0) :`false` "/Game/Assets/Characters/Idle.Idle" :`true` "/Game/Assets/Characters/Moving.Moving" :!type "PaperFlipbook Object Reference"))))))

(event `HandleRotation`
  (bind _velocity_x (`KismetMathLibrary.BreakVector` (`MovementComponent.Velocity` (`self.CharacterMovement`))))
  ;[1 1 1] Handle Rotation
  (`/Engine/EditorBlueprintResources/StandardMacros.CompareFloat` _velocity_x
    (:`>`
      (`Controller.SetControlRotation` (`self.GetController`) (`KismetMathLibrary.MakeRotator` 0.0 0.0 180.0) :!label _label))
    (:`==`
      (if (`self.ismovingright`)
        (goto _label)
        (else
          (`Controller.SetControlRotation` (`self.GetController`) (`KismetMathLibrary.MakeRotator` 0.0) :!label _label_2))))
    (:`<`
      (goto _label_2))))

(event `self.ReceiveAnyDamage`
  (params (Damage :type "Float (single-precision)") (DamageType :type "DamageType Object Reference") (InstigatedBy :type "Controller Object Reference") (DamageCauser :type "Actor Object Reference"))
  ;[1 1 1] Handle Damage
  (set `self.isdeath` true)
  (`ActorComponent.SetActive` (`self.CharacterMovement`) false false)
  (`KismetSystemLibrary.Delay` (- (`PaperFlipbook.GetTotalDuration` (`self.playerdeathanimation`)) 0.1))
  (`self.RespawnPlayerCharacter`)
  (set `self.health ` (- (`self.health `) Damage)))

(event `RespawnPlayerCharacter`
  ;[1 1 1] Respawn player
  (`self.K2_SetActorLocation` (`self.RespawnLocation`))
  (set `self.isdeath` false)
  (`ActorComponent.SetActive` (`self.CharacterMovement`) true false))

(event `self.ReceiveBeginPlay`
  ;[1 1 1] Event begin play ]
  (set `self.RespawnLocation` (`self.K2_GetActorLocation`))
  (bind _returnvalue (`|CreateWidget` "/Game/UI/Playerhud.Playerhud_C"))
  (bind _output_get (set `self.Playerhud` _returnvalue))
  (`UserWidget.AddToViewport` _output_get 0)
  (`GameplayStatics.PlaySound2D` "/Game/sounds/time_for_adventure.time_for_adventure" 1.0 1.0 0.0 null null))

(fn `UserConstructionScript`)